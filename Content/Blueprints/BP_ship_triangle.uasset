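; Player-controlled ship pawn with physics thrust and projectile shooting for a game that uses the FFA game mode.
; Turn input applies yaw both directly and through ShipMovement; throttle pushes the Box along the arrow's forward and along world X, toggling engine particles.
; Shot spawns BP_Projectile from the arrow with a gun offset, limited by a cooldown timer.
; Destruction notifies BP_gamemode_FFA.
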(event OnComponentActivated(FloatingPawnMovement)
  (params (Component :type Actor%20Component%20Object%20Reference) (bReset :type Boolean))
  ;[1 1 1] Init component values from params (speed...)
  (bind _asfloating_pawn_movement (Utilities|Casting|CastToFloatingPawnMovement Component))
  (Variables|/Script/Engine.FloatingPawnMovement|SetMaxSpeed _asfloating_pawn_movement (Variables|ShipInfo|GetEnginePower)))

(event Custom|ShootTimer
  ;[1 1 1] Shooting
  (Variables|ShipInfo|SetCanShoot true))

(event Custom|ShipMovement
  (params (AxisValue :type Float%20%28single-precision%29))
  ;[1 1 1] Rotation
  (Transformation|AddActorLocalRotation (Math|Rotator|MakeRotator 0.0 0.0 AxisValue) false false))

(event Custom|ShipThrottle
  (params (AxisValue :type Float%20%28single-precision%29))
  ;[1 1 1] Throttle
  ;[1 1 1] Thruster
  (Physics|AddForce (Variables|Default|GetBox) (* (Math|Vector|GetForwardVector (Transformation|GetWorldRotation (Variables|Default|GetArrow))) (* AxisValue (Variables|ShipInfo|GetEnginePower))) "None" false))

(event EventBeginPlay)

(event Collision|EventActorBeginOverlap
  (params (OtherActor :type Actor%20Object%20Reference)))

(event EventTick
  (params (DeltaSeconds :type Float%20%28single-precision%29)))

(event EventDestroyed
  (bind _asbp_gamemode_ffa (Utilities|Casting|CastToBP_gamemode_FFA (Game|GetGameMode)))
  (Default|OnPawnDestroyed _asbp_gamemode_ffa))

(event Input|ActionEvents|InputActionShot
  (params (Key :type Key%20Structure :default "None"))
  (bind _self self)
  (bind _arrow (Variables|Default|GetArrow))
  (bind _returnvalue (Transformation|GetWorldRotation _arrow))
  ;[1 1 1] Shooting
  (:Pressed
    (if (Variables|ShipInfo|GetCanShoot)
      (Variables|ShipInfo|SetCanShoot false)
      (Game|SpawnActorfromClass "/Game/Blueprints/BP_Projectile.BP_Projectile_C" (Math|Transform|MakeTransform (+ (Transformation|GetWorldLocation _arrow) (Math|Vector|RotateVector (Variables|GunInfo|GetGunOffset) _returnvalue)) _returnvalue) "Undefined" _self (Variables|GunInfo|GetProjectileSpeed) (Variables|GunInfo|GetProjectileLifeTime) _self)
      (Audio|PlaySound2D "/Engine/VREditor/Sounds/UI/Click_on_Button.Click_on_Button" 1.0 1.0 0.0 0 0)
      (Utilities|Time|SetTimerbyFunctionName _self "ShootTimer" 0.3))))

(event Input|AxisEvents|InputAxisThrottle
  (params (AxisValue :type Float%20%28single-precision%29))
  (bind _particlesystem (Variables|Default|GetParticleSystem))
  ;[1 1 1] Throttle
  ;;[1 1 1] Ship movement
  (CallFunction|ShipThrottle AxisValue)
  ;[1 1 1] Thruster
  (Physics|AddForce (Variables|Default|GetBox) (* "1.000000, 0, 0" (* AxisValue (Variables|ShipInfo|GetEnginePower))) "None" false)
  ;;[1 1 1] Engine particles
  (if (== AxisValue 0.0)
    (Components|Activation|Deactivate _particlesystem)
    (else
      (Components|Activation|Activate _particlesystem false))))

(event Input|AxisEvents|InputAxisTurn
  (params (AxisValue :type Float%20%28single-precision%29))
  ;[1 1 1] Rotation
  (CallFunction|ShipMovement AxisValue)
  (Transformation|AddActorLocalRotation (Math|Rotator|MakeRotator 0.0 0.0 AxisValue) false false))

(fn ConstructionScript)